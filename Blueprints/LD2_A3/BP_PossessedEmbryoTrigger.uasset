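; One-shot trigger box that makes a referenced possessed embryo actor levitate when an overlap begins.
; A timeline, scaled by ZDirection, offsets the embryo's Z from its starting location using teleport moves, with laugh sounds at start and end.
; When the timeline finishes, optional flags fire the OnPossessedEmbryoManifestEnd dispatcher to notify listeners, then destroy the embryo.
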(event OnComponentBeginOverlap(Box)
  (params (OverlappedComponent :type Primitive%20Component%20Object%20Reference) (OtherActor :type Actor%20Object%20Reference) (OtherComp :type Primitive%20Component%20Object%20Reference) (OtherBodyIndex :type Integer) (bFromSweep :type Boolean) (SweepResult :type Hit%20Result%20Structure%20%28by%20ref%29))
  (bind __possessedembryo (Variables|Default|Get_possessedEmbryo))
  (bind _defaultsceneroot (Variables|/Game/Blueprints/LD2_A3/BP_PossesedEmbryo.BP_PossesedEmbryo_C|GetDefaultSceneRoot __possessedembryo))
  ;[0 1 0.4375] Levitates Possessed embryo. Can destroy it at the end. Can call a event dispatcher at the end to notify the event
  (Utilities|FlowControl|DoOnce false
    (:Completed
      (bind _output_get (Variables|Default|Set_initialWorldLocation (Transformation|GetWorldLocation (Variables|/Game/Blueprints/LD2_A3/BP_PossesedEmbryo.BP_PossesedEmbryo_C|GetDefaultSceneRoot (Variables|Default|Get_possessedEmbryo)))))
      (Audio|PlaySoundatLocation "/Game/Audio/SFX/SFX_Laugh1.SFX_Laugh1" _output_get "0, 0, 0" 1.0 1.0 0.0 0 0 0)
      (bind _levitate (Timeline|LevitateEmbryo Play)
        (:Update
          (Transformation|SetWorldLocation _defaultsceneroot (Math|Vector|MakeVector (.x (Variables|Default|Get_initialWorldLocation)) (.y (Variables|Default|Get_initialWorldLocation)) (+ (* _levitate (Variables|Default|Get_zDirection)) (.z (Variables|Default|Get_initialWorldLocation)))) false true))
        (:Finished
          (Audio|PlaySoundatLocation "/Game/Audio/SFX/SFX_laugh2.SFX_laugh2" (Transformation|GetWorldLocation _defaultsceneroot) "0, 0, 0" 1.0 1.0 0.0 0 0 0)
          (Utilities|FlowControl|Sequence
            (:then_0
              (if (Variables|Default|Get_callDispatcher)
                (Default|CallOnPossessedEmbryoManifestEnd)))
            (:then_1
              (if (Variables|Default|Get_destroyAtEnd)
                (Actor|DestroyActor (Variables|Default|Get_possessedEmbryo))))))))))

(fn ConstructionScript)