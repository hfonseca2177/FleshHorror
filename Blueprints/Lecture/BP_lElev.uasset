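; BP_lElev is an interactable elevator that travels vertically between its placed position and a Z offset set by VLocationEnd.
; A Box overlap by the player character shows a TextRender and opens a Gate, and leaving hides the text and closes it.
; OnInteract passes through that Gate into a FlipFlop that alternately plays and reverses the MoveElevator timeline, which lerps the actor's location from the start captured in the Construction Script.
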(event OnComponentBeginOverlap(Box)
  (params (OverlappedComponent :type Primitive%20Component%20Object%20Reference) (OtherActor :type Actor%20Object%20Reference) (OtherComp :type Primitive%20Component%20Object%20Reference) (OtherBodyIndex :type Integer) (bFromSweep :type Boolean) (SweepResult :type Hit%20Result%20Structure%20%28by%20ref%29))
  (bind _v_locationstart (Variables|Default|Getv_locationStart))
  (bind (_x _y _z) (Math|Vector|BreakVector _v_locationstart))
  (if (== OtherActor (Game|GetPlayerCharacter 0))
    (Rendering|SetVisibility (Variables|Default|GetTextRender) true false)
    (Utilities|FlowControl|Gate true) ; enters at Open
  ))

(event OnComponentEndOverlap(Box)
  (params (OverlappedComponent :type Primitive%20Component%20Object%20Reference) (OtherActor :type Actor%20Object%20Reference) (OtherComp :type Primitive%20Component%20Object%20Reference) (OtherBodyIndex :type Integer))
  (bind _v_locationstart (Variables|Default|Getv_locationStart))
  (bind (_x _y _z) (Math|Vector|BreakVector _v_locationstart))
  (if (== (Game|GetPlayerCharacter 0) OtherActor)
    (Rendering|SetVisibility (Variables|Default|GetTextRender) false false)
    (Utilities|FlowControl|Gate true) ; enters at Close
  ))

(event EventOnInteract
  (bind _v_locationstart (Variables|Default|Getv_locationStart))
  (bind (_x _y _z) (Math|Vector|BreakVector _v_locationstart))
  (Utilities|FlowControl|Gate true
    (:Exit
      (Utilities|FlowControl|FlipFlop
        (:A
          (bind _move (Timeline|MoveElevator Play)
            (:Update
              (Transformation|SetActorLocation (Math|Vector|Lerp(Vector) _v_locationstart (Math|Vector|MakeVector _x _y (+ _z (Variables|Default|Getv_locationEnd))) _move) false true))))
        (:B
          (Timeline|MoveElevator Reverse))))))

(fn ConstructionScript
  (Variables|Default|Setv_locationStart (Transformation|GetActorLocation)))