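; BP_door is an interactable door that plays its open animation when used, or a handle-shake animation when locked.
; OnInteract calls OpenDoor, which branches on IsLocked and uses a DoOnce so the skeletal mesh opens only once, with no closing logic.
; A box overlap toggles the mesh's interactable highlight, and SetDoorLocked sets the lock state.
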(event OnComponentBeginOverlap(Box)
  (params (OverlappedComponent :type Primitive%20Component%20Object%20Reference) (OtherActor :type Actor%20Object%20Reference) (OtherComp :type Primitive%20Component%20Object%20Reference) (OtherBodyIndex :type Integer) (bFromSweep :type Boolean) (SweepResult :type Hit%20Result%20Structure%20%28by%20ref%29))
  ;[1 1 1] Enable Disable highlight
  (CallFunction|SwitchInteractableHighlight (Variables|Default|GetDoorSkeletalMesh) true))

(event OnComponentEndOverlap(Box)
  (params (OverlappedComponent :type Primitive%20Component%20Object%20Reference) (OtherActor :type Actor%20Object%20Reference) (OtherComp :type Primitive%20Component%20Object%20Reference) (OtherBodyIndex :type Integer))
  ;[1 1 1] Enable Disable highlight
  (CallFunction|SwitchInteractableHighlight (Variables|Default|GetDoorSkeletalMesh) false))

(event Custom|OpenDoor
  ;[1 1 1] Open/Close Door
  (if (not (Variables|Door|GetIsLocked))
    (Utilities|FlowControl|DoOnce false
      (:Completed
        (Components|Animation|PlayAnimation (Variables|Default|GetDoorSkeletalMesh) "/Game/Art/Animation/Anim_Door_CompositeOpen.Anim_Door_CompositeOpen" false)))
    (else
      (Components|Animation|PlayAnimation (Variables|Default|GetDoorSkeletalMesh) "/Game/Art/Animation/Anim_Door_HandleShake.Anim_Door_HandleShake" false))))

(event EventOnInteract
  ;[1 1 1] Interface
  (CallFunction|OpenDoor))

(fn ConstructionScript)

(fn SetDoorLocked
  (params (IsLocked :type Boolean))
  (Variables|Door|SetIsLocked IsLocked))