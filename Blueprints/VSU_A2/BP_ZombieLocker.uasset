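; Interactable locker that shakes when approached and releases an embryo when used, as a one-time scare.
; Box overlap highlights the door and runs a timeline shaking the locker vertically, restoring its location on finish or overlap end.
; Interacting fires once, enabling door physics and starting a timeline that lerps the embryo between its start location and a point above the player's live position.
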(event OnComponentBeginOverlap(Box)
  (params (OverlappedComponent :type Primitive%20Component%20Object%20Reference) (OtherActor :type Actor%20Object%20Reference) (OtherComp :type Primitive%20Component%20Object%20Reference) (OtherBodyIndex :type Integer) (bFromSweep :type Boolean) (SweepResult :type Hit%20Result%20Structure%20%28by%20ref%29))
  (bind _locker (Variables|Default|GetLocker))
  ;[1 1 1] On Everlap , highlight and shakes the locker
  (CallFunction|SwitchInteractableHighlight (Variables|Default|GetDoor) true)
  (Variables|Default|Set_originalLocation (Transformation|GetWorldLocation (Variables|Default|GetLocker)))
  (bind _shake (Timeline|ShakeTimeline Play)
    (:Update
      (Transformation|SetWorldLocation _locker (Math|Vector|MakeVector (.x (Variables|Default|Get_originalLocation)) (.y (Variables|Default|Get_originalLocation)) (+ (* _shake (Variables|Default|Get_shakeIntensity)) (.z (Variables|Default|Get_originalLocation)))) false true))
    (:Finished
      (Transformation|SetWorldLocation _locker (Variables|Default|Get_originalLocation) false false))))

(event OnComponentEndOverlap(Box)
  (params (OverlappedComponent :type Primitive%20Component%20Object%20Reference) (OtherActor :type Actor%20Object%20Reference) (OtherComp :type Primitive%20Component%20Object%20Reference) (OtherBodyIndex :type Integer))
  ;[1 1 1] Finish overlap, restoring location after shake and highlight state
  (CallFunction|SwitchInteractableHighlight (Variables|Default|GetDoor) false)
  (Transformation|SetWorldLocation (Variables|Default|GetLocker) (Variables|Default|Get_originalLocation) false false))

(event EventOnInteract
  ;[1 1 1] Interact with locker and Triggers embryo inside
  (Utilities|FlowControl|DoOnce false
    (:Completed
      (Variables|Default|Set_embryoStartLocation (Transformation|GetWorldLocation (Variables|Default|GetMesh_Embryo)))
      (Physics|SetSimulatePhysics (Variables|Default|GetDoor) true)
      (bind _move (Timeline|MoveEmbryo Play)
        (:Update
          (Transformation|SetWorldLocation (Variables|Default|GetMesh_Embryo) (Math|Vector|Lerp(Vector) (+ (Transformation|GetActorLocation (Game|GetPlayerCharacter 0)) "0, 0,150.000000") (Variables|Default|Get_embryoStartLocation) _move) false false))))))

(fn ConstructionScript)