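; BP_Collectable is a pickup actor that shows its name and a press instruction when something overlaps its box.
; On BeginPlay it writes the configured CollectableName into a text render.
; Box begin and end overlap toggle the mesh highlight and both labels, with no check on the overlapping actor.
; OnCollect prints a confirmation and destroys the actor, without adding it to any inventory.
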(event OnComponentBeginOverlap(Box)
  (params (OverlappedComponent :type Primitive%20Component%20Object%20Reference) (OtherActor :type Actor%20Object%20Reference) (OtherComp :type Primitive%20Component%20Object%20Reference) (OtherBodyIndex :type Integer) (bFromSweep :type Boolean) (SweepResult :type Hit%20Result%20Structure%20%28by%20ref%29))
  ;[1 1 1] On Overlap toggles highlight and Label
  (CallFunction|SwitchInteractableHighlight (Variables|Default|GetStaticMesh) true)
  (CallFunction|ToggleCollectableName true))

(event OnComponentEndOverlap(Box)
  (params (OverlappedComponent :type Primitive%20Component%20Object%20Reference) (OtherActor :type Actor%20Object%20Reference) (OtherComp :type Primitive%20Component%20Object%20Reference) (OtherBodyIndex :type Integer))
  ;[1 1 1] On Overlap toggles highlight and Label
  (CallFunction|SwitchInteractableHighlight (Variables|Default|GetStaticMesh) false)
  (CallFunction|ToggleCollectableName false))

(event EventBeginPlay
  ;[1 1 1] Sets Collectable Name Label
  (CallFunction|SetCollectableName))

(event EventOnCollect
  ;[1 1 1] Process Collect Input call and remove object from game
  (Development|PrintString "Item Collected")
  (Actor|DestroyActor))

(fn ConstructionScript)

(fn SetCollectableName
  ;[1 1 1] Sets the Configured collectable Name to the Text Render
  (Rendering|Components|TextRender|SetText (Variables|Default|GetTextRender) (Utilities|Text|ToText(String) (Variables|Default|GetcollectableName))))

(fn ToggleCollectableName
  (params (show :type Boolean))
  ;[1 1 1] Toggles Collectable Name Label visible
  (Rendering|SetVisibility (Variables|Default|GetTextRender) show false)
  (Rendering|SetVisibility (Variables|Default|GetPressInstruction) show false))