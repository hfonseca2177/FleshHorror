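; BP_Fireable is an object that ignites once when its linked FireTrigger fires.
; On BeginPlay it binds to the FireTrigger's OnFireTrigger dispatcher if that reference is valid, and a DoOnce lets only the first broadcast through.
; SpawnFireParticle then reveals its particle system, spawns an explosion emitter at that location and plays a non-spatialized explosion sound.
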(event Custom|OnFireTriggerEvent
  ;[1 1 1] Subscribe to the Fire Trigger On Fire Event dispatcher and execute the VFX/SFX if triggered
  (Utilities|FlowControl|DoOnce false
    (:Completed
      (CallFunction|SpawnFireParticle))))

(event EventBeginPlay
  (bind __firetrigger (Variables|Default|Get_fireTrigger))
  ;[1 1 1] Subscribe to the Fire Trigger On Fire Event dispatcher and execute the VFX/SFX if triggered
  (Utilities|IsValid __firetrigger
    (:Is%20Valid
      (EventDispatchers|AssignOnFireTrigger __firetrigger (delegate Custom|OnFireTriggerEvent)))))

(fn ConstructionScript)

(fn SpawnFireParticle
  (bind _particlesystem (Variables|Default|GetParticleSystem))
  ;[0.4062 0 1] Sequence of VFX/SFX after fire up is triggered for the given BP_fireable instance
  (Rendering|SetVisibility _particlesystem true false)
  (Effects|SpawnEmitteratLocation "/Game/Art/Particles/Systems/P_Explosion.P_Explosion" (Transformation|GetWorldLocation _particlesystem))
  (Audio|PlaySound2D "/Game/Audio/SFX/SFX_Explosion02.SFX_Explosion02" 1.0 1.0 0.0 0 0))