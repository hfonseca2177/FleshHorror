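; BP_Recorder is an interactable recorder prop that plays a short effect when the player interacts with it.
; OnInteract plays a death sound and a lightning strike at the recorder's location and flashes a point light for 0.4 seconds.
; A box trigger toggles custom depth on the recorder mesh on overlap to drive a post-process highlight.
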(event OnComponentBeginOverlap(Box)
  (params (OverlappedComponent :type Primitive%20Component%20Object%20Reference) (OtherActor :type Actor%20Object%20Reference) (OtherComp :type Primitive%20Component%20Object%20Reference) (OtherBodyIndex :type Integer) (bFromSweep :type Boolean) (SweepResult :type Hit%20Result%20Structure%20%28by%20ref%29))
  ;[0.875 1 0] Enable and disable Highlight posprocessing effect to an interactable object
  (Rendering|SetRenderCustomDepth (Variables|Default|GetRecorder) true))

(event OnComponentEndOverlap(Box)
  (params (OverlappedComponent :type Primitive%20Component%20Object%20Reference) (OtherActor :type Actor%20Object%20Reference) (OtherComp :type Primitive%20Component%20Object%20Reference) (OtherBodyIndex :type Integer))
  ;[0.875 1 0] Enable and disable Highlight posprocessing effect to an interactable object
  (Rendering|SetRenderCustomDepth (Variables|Default|GetRecorder) false))

(event EventOnInteract
  (bind _recorder (Variables|Default|GetRecorder))
  (bind _pointlight (Variables|Default|GetPointLight))
  (bind _returnvalue (Transformation|GetWorldLocation _recorder))
  ;[0 0.03906 1] Play Recorder content with some FXs
  (Audio|PlaySoundatLocation "/Game/Audio/SFX/SFX_PlayerDeathShort_Cue.SFX_PlayerDeathShort_Cue" _returnvalue "0, 0, 0" 1.0 1.0 0.0 0 0 0)
  (Audio|PlaySoundatLocation "/Game/Audio/SFX/SFX_LightningStrike01.SFX_LightningStrike01" _returnvalue "0, 0, 0" 1.0 1.0 0.0 0 0 0)
  (Rendering|SetVisibility _pointlight true false)
  (Utilities|FlowControl|Delay 0.4)
  (Rendering|SetVisibility _pointlight false false))

(fn ConstructionScript)