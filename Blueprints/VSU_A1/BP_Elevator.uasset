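; Interactable elevator that alternates between moving up and back down on each interaction while the player stands in its trigger box.
; Box overlaps open or close a gate for the player and toggle the floor's interactable highlight for any overlapping actor.
; A FlipFlop plays or reverses a timeline that lerps the actor from its construction-time location along Z by LocationZEnd, with start and stop sounds.
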(event OnComponentBeginOverlap(Box)
  (params (OverlappedComponent :type Primitive%20Component%20Object%20Reference) (OtherActor :type Actor%20Object%20Reference) (OtherComp :type Primitive%20Component%20Object%20Reference) (OtherBodyIndex :type Integer) (bFromSweep :type Boolean) (SweepResult :type Hit%20Result%20Structure%20%28by%20ref%29))
  (bind __locationstart (Variables|Default|Get_locationStart))
  (bind (_x _y _z) (Math|Vector|BreakVector __locationstart))
  ;[0 0.1562 1] Manages elevator functions to move up and down if activated by the player
  (Utilities|FlowControl|Sequence
    (:then_0
      (if (== OtherActor (Game|GetPlayerCharacter 0))
        (Utilities|FlowControl|Gate true) ; enters at Open
      ))
    (:then_1
      (CallFunction|SwitchInteractableHighlight (Variables|Default|GetFloor) true))))

(event OnComponentEndOverlap(Box)
  (params (OverlappedComponent :type Primitive%20Component%20Object%20Reference) (OtherActor :type Actor%20Object%20Reference) (OtherComp :type Primitive%20Component%20Object%20Reference) (OtherBodyIndex :type Integer))
  (bind __locationstart (Variables|Default|Get_locationStart))
  (bind (_x _y _z) (Math|Vector|BreakVector __locationstart))
  ;[0 0.1562 1] Manages elevator functions to move up and down if activated by the player
  (Utilities|FlowControl|Sequence
    (:then_0
      (if (== (Game|GetPlayerCharacter 0) OtherActor)
        (Utilities|FlowControl|Gate true) ; enters at Close
      ))
    (:then_1
      (CallFunction|SwitchInteractableHighlight (Variables|Default|GetFloor) false))))

(event EventOnInteract
  (bind __locationstart (Variables|Default|Get_locationStart))
  (bind (_x _y _z) (Math|Vector|BreakVector __locationstart))
  ;[0 0.1562 1] Manages elevator functions to move up and down if activated by the player
  (Utilities|FlowControl|Gate true
    (:Exit
      (Audio|PlaySound2D "/Game/Audio/SFX/SFX_ElevatorStart.SFX_ElevatorStart" 1.0 1.0 0.0 0 0)
      (Utilities|FlowControl|FlipFlop
        (:A
          (bind _movenormalizedvalue (Timeline|MoveTimeline PlayFromStart)
            (:Update
              (Transformation|SetActorLocation (Math|Vector|Lerp(Vector) __locationstart (Math|Vector|MakeVector _x _y (+ _z (Variables|Default|Get_locationZEnd))) _movenormalizedvalue) false true))
            (:Finished
              (Audio|PlaySound2D "/Game/Audio/SFX/SFX_ElevatorStop.SFX_ElevatorStop" 1.0 1.0 0.0 0 0))))
        (:B
          (Timeline|MoveTimeline Reverse))))))

(fn ConstructionScript
  (Variables|Default|Set_locationStart (Transformation|GetActorLocation)))