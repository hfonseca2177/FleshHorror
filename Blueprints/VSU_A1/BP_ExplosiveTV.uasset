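; Interactable TV that explodes when the player interacts with it.
; On interact it hides the TVOn mesh, reveals the TVOff mesh and calls PlayTVExplosionFX, which spawns spark and smoke emitters and plays an explosion sound at the TVOff location.
; A Box overlap toggles the interactable highlight on the TVOn mesh only.
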(event OnComponentBeginOverlap(Box)
  (params (OverlappedComponent :type Primitive%20Component%20Object%20Reference) (OtherActor :type Actor%20Object%20Reference) (OtherComp :type Primitive%20Component%20Object%20Reference) (OtherBodyIndex :type Integer) (bFromSweep :type Boolean) (SweepResult :type Hit%20Result%20Structure%20%28by%20ref%29))
  ;[1 0.8906 0] Enable Disable highlight on interactable
  ; - For this case, enable only for tvOn mesh
  (CallFunction|SwitchInteractableHighlight (Variables|Default|GetTVOn) true))

(event OnComponentEndOverlap(Box)
  (params (OverlappedComponent :type Primitive%20Component%20Object%20Reference) (OtherActor :type Actor%20Object%20Reference) (OtherComp :type Primitive%20Component%20Object%20Reference) (OtherBodyIndex :type Integer))
  ;[1 0.8906 0] Enable Disable highlight on interactable
  ; - For this case, enable only for tvOn mesh
  (CallFunction|SwitchInteractableHighlight (Variables|Default|GetTVOn) false))

(event EventOnInteract
  (bind _tvoff (Variables|Default|GetTVOff))
  (bind _returnvalue (Transformation|GetWorldLocation _tvoff))
  ;[0.5703 0 1] On interact swap meshes and play FX for TV destruction
  (Development|SetHiddeninGame (Variables|Default|GetTVOn) true true)
  (Development|SetHiddeninGame _tvoff false false)
  (CallFunction|PlayTVExplosionFX _returnvalue _returnvalue _returnvalue))

(fn ConstructionScript)

(fn PlayTVExplosionFX
  (params (Location :type Vector) (Location2 :type Vector) (Location3 :type Vector))
  ;[1 0 0.75] FX sequences for trying to interact with the TV
  (Utilities|FlowControl|Sequence
    (:then_0
      (Effects|SpawnEmitteratLocation "/Game/Art/Particles/Systems/P_Sparks.P_Sparks" Location))
    (:then_1
      (Effects|SpawnEmitteratLocation "/Game/Art/Particles/Systems/P_Smoke.P_Smoke" Location2))
    (:then_2
      (Audio|PlaySoundatLocation "/Game/Audio/SFX/SFX_Explosion01.SFX_Explosion01" Location3 "0, 0, 0" 1.0 1.0 0.0 0 0 0))))